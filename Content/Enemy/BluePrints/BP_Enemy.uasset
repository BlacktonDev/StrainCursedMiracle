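; BP_Enemy is an enemy Blueprint whose look-at effect on its Manny animation can be switched on and off.
; On BeginPlay it stores its starting location as Origin and caches the mesh's ABP_Manny anim instance.
; LookAtActive and LookAtDeactivate drive that instance's Alpha through two separate timelines, one played forward and the other reversed.
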(event Custom|LookAtActive
  (bind _newtrack_0 (Timeline|Timeline Play)
    (:Update
      (Variables|/Game/Characters/Mannequins/Animations/ABP_Manny.ABP_Manny_C|SetAlpha (Variables|Default|GetAs%20ABP%20Manny) _newtrack_0))))

(event Custom|LookAtDeactivate
  (bind _newtrack_0 (Timeline|Timeline_0 Reverse)
    (:Update
      (Variables|/Game/Characters/Mannequins/Animations/ABP_Manny.ABP_Manny_C|SetAlpha (Variables|Default|GetAs%20ABP%20Manny) _newtrack_0))))

(event EventBeginPlay
  (bind _mesh (Variables|Character|GetMesh))
  (bind _returnvalue (Components|SkeletalMesh|GetAnimInstance _mesh))
  (bind _asabp_manny (Utilities|Casting|CastToABP_Manny _returnvalue))
  (Variables|Default|SetOrigin (Transformation|GetActorLocation))
  (Utilities|IsValid _asabp_manny
    (:Is%20Valid
      (Variables|Default|SetAs%20ABP%20Manny _asabp_manny))))

(event Collision|EventActorBeginOverlap
  (params (OtherActor :type Actor%20Object%20Reference)))

(event EventTick
  (params (DeltaSeconds :type Float%20%28single-precision%29)))

(fn ConstructionScript)
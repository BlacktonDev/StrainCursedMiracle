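; Rifle weapon Blueprint that adds automatic fire to its parent weapon class.
; StartShooting fires at once and, if Playanimation is set, animates the gun mesh and starts a looping timer at Firerate.
; Each timer tick fires again, playing the gun animation plus a first-person hands montage while Playanimation holds.
; The timer clears when Playanimation is false on a tick or StopShooting runs.
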(event Custom|Fire%20rifle
  (CallFunction|Fireweapon)
  (if (Variables|Default|Getplayanimation?)
    (Components|Animation|PlayAnimation (Variables|Default|GetGunmesh) "/Game/MilitaryWeapSilver/Weapons/Animations/Fire_Rifle_W.Fire_Rifle_W" false)
    (Animation|Montage|PlayMontage (Variables|/Game/blueprints/fpscharacter_bp.fpscharacter_bp_C|GetFPSHands (Variables|Default|Getplayerref)) "/Game/Man/Demo/Animations/FiringRifle_UE_Montage.FiringRifle_UE_Montage")
    (else
      (Utilities|Time|ClearandInvalidateTimerbyHandle (Variables|Default|GetFirevent)))))

(event EventStartShooting
  (CallFunction|Fireweapon)
  (if (Variables|Default|Getplayanimation?)
    (Components|Animation|PlayAnimation (Variables|Default|GetGunmesh) "/Game/MilitaryWeapSilver/Weapons/Animations/Fire_Rifle_W.Fire_Rifle_W" false)
    (bind _returnvalue (Utilities|Time|SetTimerbyEvent (delegate Custom|Fire%20rifle) (Variables|Default|Getfirerate) true))
    (Variables|Default|SetFirevent _returnvalue)))

(event EventStopShooting
  (Utilities|Time|ClearandInvalidateTimerbyHandle (Variables|Default|GetFirevent)))

(fn ConstructionScript
  (|CallParentFunction))
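; Weapon pickup actor that swaps the player's currently held weapon for the one it carries when interacted with.
; Interact checks whether the main or secondary slot is equipped, spawns a new pickup holding that weapon, then writes its own weapon and ammo into the slot.
; It then sets the character's weapon child actor class, refreshes HUD and ammo, and destroys itself.
; The construction script picks the skeletal mesh from the weapon class's default name.
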(event EventBeginPlay
  (bind _asfpscharacter_bp (Utilities|Casting|CastTofpscharacter_bp (Game|GetPlayerCharacter 0)))
  (Variables|Default|SetAs%20Fpscharacter%20Bp _asfpscharacter_bp))

(event EventInteract
  (bind _as_fpscharacter_bp (Variables|Default|GetAs%20Fpscharacter%20Bp))
  (bind _as_fpscharacter_bp_2 (Variables|Default|GetAs%20Fpscharacter%20Bp))
  (bind _weapon (Variables|Default|GetWeapon))
  (bind _weapon_2 (Variables|Default|GetWeapon))
  (bind _as_fpscharacter_bp_3 (Variables|Default|GetAs%20Fpscharacter%20Bp))
  (bind _as_fpscharacter_bp_4 (Variables|Default|GetAs%20Fpscharacter%20Bp))
  (bind _weapon_3 (Variables|Default|GetWeapon))
  (bind _weapon_4 (Variables|Default|GetWeapon))
  (bind _as_fpscharacter_bp_5 (Variables|Default|GetAs%20Fpscharacter%20Bp))
  (bind _weaponref (Variables|/Game/blueprints/fpscharacter_bp.fpscharacter_bp_C|Getweaponref _as_fpscharacter_bp_2))
  (bind _weaponref_2 (Variables|/Game/blueprints/fpscharacter_bp.fpscharacter_bp_C|Getweaponref _as_fpscharacter_bp_4))
  ;[1 1 1] Swap weapon when player interacts
  (if (== (Variables|/Script/Engine.ChildActorComponent|GetChildActorClass (Variables|/Game/blueprints/fpscharacter_bp.fpscharacter_bp_C|Getweapon _as_fpscharacter_bp)) (.weapon (Variables|/Game/blueprints/fpscharacter_bp.fpscharacter_bp_C|GetMainweapon _as_fpscharacter_bp)))
    (Game|SpawnActorfromClass "Weaponpickup_BP_C" (Transformation|GetActorTransform) "Undefined" "MultiplyWithRoot" 0 (Variables|/Game/blueprints/fpscharacter_bp.fpscharacter_bp_C|GetMainweapon (Variables|Default|GetAs%20Fpscharacter%20Bp)) 0)
    (Variables|/Game/blueprints/fpscharacter_bp.fpscharacter_bp_C|SetMainweapon (Variables|Default|GetAs%20Fpscharacter%20Bp) (Utilities|Struct|MakeWeaponStruct (.weapon _weapon_2) (.currentammo _weapon_2) (.maxammo _weapon_2)))
    (Widget|RemovefromParent (Variables|/Game/blueprints/fpscharacter_bp.fpscharacter_bp_C|Getplayerhudref _as_fpscharacter_bp_3))
    (ChildActorComponent|SetChildActorClass (Variables|/Game/blueprints/fpscharacter_bp.fpscharacter_bp_C|Getweapon _as_fpscharacter_bp_3) (.weapon (Variables|Default|GetWeapon)))
    (Default|Update (Variables|Default|GetAs%20Fpscharacter%20Bp))
    (Variables|/Game/blueprints/weapons/Baseweapon_BP.Baseweapon_BP_C|Setcurrentammo _weaponref_2 (.currentammo _weapon_3))
    (Variables|/Game/blueprints/weapons/Baseweapon_BP.Baseweapon_BP_C|Setmaxammo _weaponref_2 (.maxammo _weapon_3))
    (Actor|DestroyActor)
    (else
      (Game|SpawnActorfromClass "Weaponpickup_BP_C" (Transformation|GetActorTransform) "Undefined" "MultiplyWithRoot" 0 (Variables|/Game/blueprints/fpscharacter_bp.fpscharacter_bp_C|GetSecondaryweapon (Variables|Default|GetAs%20Fpscharacter%20Bp)) 0)
      (Variables|/Game/blueprints/fpscharacter_bp.fpscharacter_bp_C|SetSecondaryweapon (Variables|Default|GetAs%20Fpscharacter%20Bp) (Utilities|Struct|MakeWeaponStruct (.weapon _weapon_4) (.currentammo _weapon_4) (.maxammo _weapon_4)))
      (Widget|RemovefromParent (Variables|/Game/blueprints/fpscharacter_bp.fpscharacter_bp_C|Getplayerhudref _as_fpscharacter_bp_5))
      (ChildActorComponent|SetChildActorClass (Variables|/Game/blueprints/fpscharacter_bp.fpscharacter_bp_C|Getweapon _as_fpscharacter_bp_5) (.weapon (Variables|Default|GetWeapon)))
      (Default|Update (Variables|Default|GetAs%20Fpscharacter%20Bp))
      (Variables|/Game/blueprints/weapons/Baseweapon_BP.Baseweapon_BP_C|Setcurrentammo _weaponref (.currentammo _weapon))
      (Variables|/Game/blueprints/weapons/Baseweapon_BP.Baseweapon_BP_C|Setmaxammo _weaponref (.maxammo _weapon))
      (Actor|DestroyActor))))

(fn ConstructionScript
  (switch string (Utilities|String|ToString(Text) (.Weaponname (Utilities|GetClassDefaults (.weapon (Variables|Default|GetWeapon)))))
    (:Pistol
      (Components|SkeletalMesh|SetSkeletalMeshAsset (Variables|Default|GetSkeletalMesh) "/Game/MilitaryWeapSilver/Weapons/Pistols_A.Pistols_A"))
    (:Rifle
      (Components|SkeletalMesh|SetSkeletalMeshAsset (Variables|Default|GetSkeletalMesh) "/Game/MilitaryWeapSilver/Weapons/Assault_Rifle_A.Assault_Rifle_A"))
    (:Shotgun
      (Components|SkeletalMesh|SetSkeletalMeshAsset (Variables|Default|GetSkeletalMesh) "/Game/MilitaryWeapSilver/Weapons/Shotgun_A.Shotgun_A"))))
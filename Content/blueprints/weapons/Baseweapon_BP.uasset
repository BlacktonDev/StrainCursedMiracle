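; Base weapon Blueprint providing hitscan firing, magazine-and-reserve reloading and iron sights, with empty start/stop shooting events.
; Iron sights blend the view to the weapon actor while Tick keeps the player camera on control rotation.
; Fireweapon traces from the active camera, spends ammo, shakes the camera and emits AI noise.
; Hits apply damage, with a head-bone multiplier and blood for zombie-tagged actors, or bullet decals and impact effects otherwise.
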(event Custom|Start%20shooting)

(event Custom|Stop%20shooting)

(event Custom|Start%20Ironsights
  ;[1 1 1] Iron sights
  (Variables|Default|SetIronsight? true)
  (Game|Player|SetViewTargetwithBlend (Game|GetPlayerController 0) self 0.16 "VTBlend_Linear" 0.0 false))

(event Custom|Stop%20ironsights
  ;[1 1 1] Iron sights
  (Variables|Default|SetIronsight? false)
  (Game|Player|SetViewTargetwithBlend (Game|GetPlayerController 0) (Game|GetPlayerCharacter 0) 0.16 "VTBlend_Linear" 0.0 false))

(event EventTick
  (params (DeltaSeconds :type Float%20%28single-precision%29))
  ;[1 1 1] When ironsights is active change players rotation
  (if (Variables|Default|GetIronsight?)
    (Transformation|SetWorldRotation (Variables|/Game/blueprints/fpscharacter_bp.fpscharacter_bp_C|GetCamera (Variables|Default|Getplayerref)) (Pawn|GetControlRotation (Game|GetPlayerController 0) :!class /Script/Engine.Controller) false false)))

(fn ConstructionScript)

(fn Fireweapon
  (bind _playerref (Variables|Default|Getplayerref))
  (bind _playerref_2 (Variables|Default|Getplayerref))
  (bind _ironsight_ (Variables|Default|GetIronsight?))
  (bind _camera (Variables|Default|GetCamera))
  (bind _camera_2 (Variables|/Game/blueprints/fpscharacter_bp.fpscharacter_bp_C|GetCamera _playerref))
  (bind _returnvalue (select _ironsight_ _camera _camera_2))
  (bind _returnvalue_2 (Transformation|GetWorldLocation _returnvalue))
  (if (> (Variables|Default|Getcurrentammo) 0)
    (Variables|Default|Setplayanimation? true)
    (Default|Camerashake (Variables|Default|Getplayerref))
    (bind _outhit (Collision|LineTraceByChannel _returnvalue_2 (+ _returnvalue_2 (* (Math|Vector|GetForwardVector _returnvalue) 3e+03)) "TraceTypeQuery1" false 0 "None"))
    ;[1 1 1] If gun hits zombie
    (Math|Integer|DecrementInt (Variables|Default|Getcurrentammo)
      (:%20%20
        (Class|PawnNoiseEmitterComponent|MakeNoise (Variables|/Game/blueprints/fpscharacter_bp.fpscharacter_bp_C|GetPawnNoiseEmitter _playerref_2) _playerref_2 1.0 (Transformation|GetActorLocation _playerref_2))
        (Utilities|IsValid (.HitActor (Collision|BreakHitResult _outhit))
          (:Is%20Valid
            (if (Actor|ActorHasTag (.HitActor (Collision|BreakHitResult _outhit)) "zombie")
              (if (== (.HitBoneName (Collision|BreakHitResult _outhit)) "Base-HumanHead")
                (Game|Damage|ApplyDamage (.HitActor (Collision|BreakHitResult _outhit)) (* (Variables|Default|Getdamage) (Variables|Default|Getheadshotmultiplyer)) 0 0)
                (else
                  (Game|Damage|ApplyDamage (.HitActor (Collision|BreakHitResult _outhit)) (Variables|Default|Getdamage) 0 0)))
              (Effects|SpawnEmitteratLocation "/Game/Realistic_Starter_VFX_Pack_Vol2/Particles/Blood/P_Blood_Splat_Cone.P_Blood_Splat_Cone" (.Location (Collision|BreakHitResult _outhit)))
              (else
                ;[1 1 1] If gun hits an object,  spawn bullet hole
                (Rendering|Decal|SpawnDecalatLocation "/Game/Images/bullet_hole_Mat.bullet_hole_Mat" "6.000000,6.000000,6.000000" (.Location (Collision|BreakHitResult _outhit)) (Math|Conversions|RotationFromXVector (.ImpactNormal (Collision|BreakHitResult _outhit))) 5.0)
                (Effects|SpawnEmitteratLocation "/Game/Realistic_Starter_VFX_Pack_Vol2/Particles/Hit/P_Default.P_Default" (.Location (Collision|BreakHitResult _outhit)))
                (Game|Damage|ApplyDamage (.HitActor (Collision|BreakHitResult _outhit)) (Variables|Default|Getdamage) 0 0)))))))
    (else
      (Variables|Default|Setplayanimation? false))))

(fn Reload
  (bind _output_get (LocalVariables|Setammodifference (- (Variables|Default|Getmagzinesize) (Variables|Default|Getcurrentammo))))
  (if (>= (Variables|Default|Getmaxammo) _output_get)
    (Variables|Default|Setcurrentammo (Variables|Default|Getmagzinesize))
    (Variables|Default|Setmaxammo (- (Variables|Default|Getmaxammo) (LocalVariables|Getammodifference)))
    (else
      (Variables|Default|Setcurrentammo (+ (Variables|Default|Getcurrentammo) (Variables|Default|Getmaxammo)))
      (Variables|Default|Setmaxammo 0))))
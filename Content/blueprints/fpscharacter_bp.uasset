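; First-person player character handling Enhanced Input movement, sprinting with stamina, interface-based interaction and damage with cooldown and game over.
; Weapons run through a child actor whose class swaps between main and secondary slots, saving ammo counts.
; Update binds each weapon to the hands mesh socket and recreates the HUD, while input forwards shooting, ironsights and montage-timed reloads.
; Portal jumps redirect velocity along the exit facing, preserving speed.
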(event Custom|Update
  (bind _mainweapon (Variables|Default|GetMainweapon))
  ;[1 1 1] Handle setting up weapons
  (bind _asbaseweapon_bp (Utilities|Casting|CastToBaseweapon_BP (Variables|/Script/Engine.ChildActorComponent|GetChildActor (Variables|Default|Getweapon))))
  (bind _output_get (Variables|Default|Setweaponref _asbaseweapon_bp))
  (Variables|/Game/blueprints/weapons/Baseweapon_BP.Baseweapon_BP_C|Setplayerref _output_get self)
  (Transformation|AttachComponentToComponent (Variables|/Game/blueprints/weapons/Baseweapon_BP.Baseweapon_BP_C|GetGunmesh (Variables|Default|Getweaponref)) (Variables|Default|GetFPSHands) (Variables|/Game/blueprints/weapons/Baseweapon_BP.Baseweapon_BP_C|GetSocket (Variables|Default|Getweaponref)) "SnapToTarget" "SnapToTarget" "SnapToTarget" true)
  (Variables|Default|SetAnim (Variables|/Game/blueprints/weapons/Baseweapon_BP.Baseweapon_BP_C|GetAnim (Variables|Default|Getweaponref)))
  (bind _returnvalue (UserInterface|CreateWidget "/Game/UI/Playerhud_WB.Playerhud_WB_C"))
  (bind _output_get_2 (Variables|Default|Setplayerhudref _returnvalue))
  (UserInterface|Viewport|AddtoViewport _output_get_2 0)
  (Utilities|FlowControl|DoOnce false
    (:Completed
      (Variables|/Game/blueprints/weapons/Baseweapon_BP.Baseweapon_BP_C|Setcurrentammo (Variables|Default|Getweaponref) (.currentammo _mainweapon))
      (Variables|/Game/blueprints/weapons/Baseweapon_BP.Baseweapon_BP_C|Setmaxammo (Variables|Default|Getweaponref) (.maxammo _mainweapon))
      (while (and (not (Variables|Default|Getissprinting?)) (<= (Variables|Default|Getstamina) 1e+02))
        (Math|Float|IncrementFloat (Variables|Default|Getstamina)))
      (Development|PrintString "STAMINA RECARGADA"))))

(event Custom|Camerashake
  ;[1 1 1] Camera shake
  (Camera|PlayWorldCameraShake "/Game/blueprints/Shoot_CS.Shoot_CS_C" (Transformation|GetActorLocation) 0.0 2e+02))

(event Input|EnhancedActionEvents|EnhancedInputActionShoot_IA
  (params (ActionValue :type Boolean) (ElapsedSeconds :type Float%20%28double-precision%29) (TriggeredSeconds :type Float%20%28double-precision%29) (InputAction :type Input%20Action%20Object%20Reference :default "/Game/Input/Shoot_IA.Shoot_IA"))
  (bind _weaponref (Variables|Default|Getweaponref))
  ;[1 1 1] Handle shooting
  (:Started
    (if (not (or (Variables|Default|GetIsreloading?) (Variables|Default|Getissprinting?)))
      (Default|StartShooting _weaponref)))
  (:Completed
    (Default|StopShooting _weaponref)))

(event Input|EnhancedActionEvents|EnhancedInputActionMove_IA
  (params (ActionValue :type Vector%202D%20Structure) (ElapsedSeconds :type Float%20%28double-precision%29) (TriggeredSeconds :type Float%20%28double-precision%29) (InputAction :type Input%20Action%20Object%20Reference :default "/Game/Input/Move_IA.Move_IA"))
  ;[1 1 1] Handle movement
  (Pawn|Input|AddMovementInput (Transformation|GetActorRightVector) (.x ActionValue) false)
  (Pawn|Input|AddMovementInput (Transformation|GetActorForwardVector) (.y ActionValue) false))

(event Input|EnhancedActionEvents|EnhancedInputActionLook_IA
  (params (ActionValue :type Vector%202D%20Structure) (ElapsedSeconds :type Float%20%28double-precision%29) (TriggeredSeconds :type Float%20%28double-precision%29) (InputAction :type Input%20Action%20Object%20Reference :default "/Game/Input/Look_IA.Look_IA"))
  ;[1 1 1] Handle camera movement
  (Pawn|Input|AddControllerYawInput (.x ActionValue))
  (Pawn|Input|AddControllerPitchInput (.y ActionValue)))

(event Input|EnhancedActionEvents|EnhancedInputActionReload_IA
  (params (ActionValue :type Boolean) (ElapsedSeconds :type Float%20%28double-precision%29) (TriggeredSeconds :type Float%20%28double-precision%29) (InputAction :type Input%20Action%20Object%20Reference :default "/Game/Input/Reload_IA.Reload_IA"))
  ;[1 0 0] Reload
  (:Started
    (Default|StopShooting (Variables|Default|Getweaponref))
    (Variables|Default|SetIsreloading? true)
    (switch int (Variables|Default|GetAnim)
      (:1
        (Animation|Montage|PlayMontage (Variables|Default|GetFPSHands) "/Game/Man/Demo/Animations/Reload_Rifle_Hip_Montage.Reload_Rifle_Hip_Montage"
          (:OnCompleted
            (Default|Reload (Variables|Default|Getweaponref))
            (Variables|Default|SetIsreloading? false)))))))

(event Input|EnhancedActionEvents|EnhancedInputActionJump_IA
  (params (ActionValue :type Boolean) (ElapsedSeconds :type Float%20%28double-precision%29) (TriggeredSeconds :type Float%20%28double-precision%29) (InputAction :type Input%20Action%20Object%20Reference :default "/Game/Input/Jump_IA.Jump_IA"))
  ;[1 1 1] Handle jumping
  (:Started
    (Character|Jump))
  (:Completed
    (Character|StopJumping)))

(event Input|EnhancedActionEvents|EnhancedInputActionIronsights_IA
  (params (ActionValue :type Boolean) (ElapsedSeconds :type Float%20%28double-precision%29) (TriggeredSeconds :type Float%20%28double-precision%29) (InputAction :type Input%20Action%20Object%20Reference :default "/Game/Input/Ironsights_IA.Ironsights_IA"))
  (bind _weaponref (Variables|Default|Getweaponref))
  (bind _playerhudref (Variables|Default|Getplayerhudref))
  ;[1 1 1] Handle ironsights
  (:Started
    (Default|StartIronsights _weaponref)
    (Default|Turncrosshairoff _playerhudref))
  (:Completed
    (Default|StopIronsights _weaponref)
    (Default|Turncrosshairon _playerhudref)))

(event Input|EnhancedActionEvents|EnhancedInputActionInteract_IA
  (params (ActionValue :type Boolean) (ElapsedSeconds :type Float%20%28double-precision%29) (TriggeredSeconds :type Float%20%28double-precision%29) (InputAction :type Input%20Action%20Object%20Reference :default "/Game/Input/Interact_IA.Interact_IA"))
  ;[1 1 1] Handle interaction
  (:Started
    (bind _array_element (Utilities|Array|ForEachLoopwithBreak (Collision|GetOverlappingActors 0 :!class /Script/Engine.Actor))
      (:LoopBody
        (if (Utilities|DoesObjectImplementInterface _array_element "/Game/blueprints/weapons/interactioninterface.interactioninterface_C")
          (Class|Interactioninterface|Interact(Message) _array_element))))))

(event Input|EnhancedActionEvents|EnhancedInputActionSwap_IA
  (params (ActionValue :type Boolean) (ElapsedSeconds :type Float%20%28double-precision%29) (TriggeredSeconds :type Float%20%28double-precision%29) (InputAction :type Input%20Action%20Object%20Reference :default "/Game/Input/Swap_IA.Swap_IA"))
  (bind _weaponref (Variables|Default|Getweaponref))
  (bind _weaponref_2 (Variables|Default|Getweaponref))
  (bind _weaponref_3 (Variables|Default|Getweaponref))
  (bind _weaponref_4 (Variables|Default|Getweaponref))
  ;[1 1 1] Swapping weapons
  (:Started
    (if (== (Variables|/Script/Engine.ChildActorComponent|GetChildActorClass (Variables|Default|Getweapon)) (.weapon (Variables|Default|GetMainweapon)))
      (Variables|Default|SetMainweapon (Utilities|Struct|MakeWeaponStruct (.weapon (Variables|Default|GetMainweapon)) (Variables|/Game/blueprints/weapons/Baseweapon_BP.Baseweapon_BP_C|Getcurrentammo _weaponref_4) (Variables|/Game/blueprints/weapons/Baseweapon_BP.Baseweapon_BP_C|Getmaxammo _weaponref_4)))
      (ChildActorComponent|SetChildActorClass (Variables|Default|Getweapon) (.weapon (Variables|Default|GetSecondaryweapon)))
      (Widget|RemovefromParent (Variables|Default|Getplayerhudref))
      (CallFunction|Update)
      (Variables|/Game/blueprints/weapons/Baseweapon_BP.Baseweapon_BP_C|Setcurrentammo _weaponref_2 (.currentammo (Variables|Default|GetSecondaryweapon)))
      (Variables|/Game/blueprints/weapons/Baseweapon_BP.Baseweapon_BP_C|Setmaxammo _weaponref_2 (.maxammo (Variables|Default|GetSecondaryweapon)))
      (else
        (Variables|Default|SetSecondaryweapon (Utilities|Struct|MakeWeaponStruct (.weapon (Variables|Default|GetSecondaryweapon)) (Variables|/Game/blueprints/weapons/Baseweapon_BP.Baseweapon_BP_C|Getcurrentammo _weaponref_3) (Variables|/Game/blueprints/weapons/Baseweapon_BP.Baseweapon_BP_C|Getmaxammo _weaponref_3)))
        (ChildActorComponent|SetChildActorClass (Variables|Default|Getweapon) (.weapon (Variables|Default|GetMainweapon)))
        (Widget|RemovefromParent (Variables|Default|Getplayerhudref))
        (CallFunction|Update)
        (Variables|/Game/blueprints/weapons/Baseweapon_BP.Baseweapon_BP_C|Setcurrentammo _weaponref (.currentammo (Variables|Default|GetMainweapon)))
        (Variables|/Game/blueprints/weapons/Baseweapon_BP.Baseweapon_BP_C|Setmaxammo _weaponref (.maxammo (Variables|Default|GetMainweapon)))))))

(event Input|EnhancedActionEvents|EnhancedInputActionSprint_IA
  (params (ActionValue :type Boolean) (ElapsedSeconds :type Float%20%28double-precision%29) (TriggeredSeconds :type Float%20%28double-precision%29) (InputAction :type Input%20Action%20Object%20Reference :default "/Game/Input/Sprint_IA.Sprint_IA"))
  (bind _playerhudref (Variables|Default|Getplayerhudref))
  ;[1 1 1] Sprint system
  (:Triggered
    (if (> (Variables|Default|Getstamina) 0.0)
      (Math|Float|DecrementFloat (Variables|Default|Getstamina)
        (:%20%20
          (if (and (> (Variables|Default|Getstamina) 0.0) (> (Math|Vector|VectorLength (Variables|/Script/Engine.MovementComponent|GetVelocity (Variables|Character|GetCharacterMovement))) 0.0))
            (Variables|Default|Setissprinting? true)
            (Variables|/Script/Engine.CharacterMovementComponent|SetMaxWalkSpeed (Variables|Character|GetCharacterMovement) (Variables|Default|GetSprintspeed))
            (Default|Turncrosshairoff _playerhudref))))))
  (:Completed
    (Variables|Default|Setissprinting? false)
    (Variables|/Script/Engine.CharacterMovementComponent|SetMaxWalkSpeed (Variables|Character|GetCharacterMovement) (Variables|Default|Getdefaultspeed))
    (Default|Turncrosshairon _playerhudref)))

(event EventBeginPlay
  (bind _returnvalue (Game|GetPlayerController 0))
  (bind _mainweapon (Variables|Default|GetMainweapon))
  (Variables|/Script/Engine.PlayerController|SetbShowMouseCursor _returnvalue false)
  ;[1 1 1] Add input controls
  (Input|SetInputModeGameOnly _returnvalue false)
  (bind _asplayer_controller (Utilities|Casting|CastToPlayerController (Pawn|GetController)))
  (Utilities|IsValid (PlayerController|LocalPlayerSubsystems|GetEnhancedInputLocalPlayerSubsystem _asplayer_controller)
    (:Is%20Valid
      (Input|AddMappingContext (PlayerController|LocalPlayerSubsystems|GetEnhancedInputLocalPlayerSubsystem _asplayer_controller) "/Game/Input/FPS_IMC.FPS_IMC" 0 "(bIgnoreAllPressedKeysUntilRelease=True,bForceImmediately=False,bNotifyUserSettings=False)")
      ;[1 1 1] Handle setting up weapons
      (ChildActorComponent|SetChildActorClass (Variables|Default|Getweapon) (.weapon (Variables|Default|GetMainweapon)))
      (bind _asbaseweapon_bp (Utilities|Casting|CastToBaseweapon_BP (Variables|/Script/Engine.ChildActorComponent|GetChildActor (Variables|Default|Getweapon))))
      (bind _output_get (Variables|Default|Setweaponref _asbaseweapon_bp))
      (Variables|/Game/blueprints/weapons/Baseweapon_BP.Baseweapon_BP_C|Setplayerref _output_get self)
      (Transformation|AttachComponentToComponent (Variables|/Game/blueprints/weapons/Baseweapon_BP.Baseweapon_BP_C|GetGunmesh (Variables|Default|Getweaponref)) (Variables|Default|GetFPSHands) (Variables|/Game/blueprints/weapons/Baseweapon_BP.Baseweapon_BP_C|GetSocket (Variables|Default|Getweaponref)) "SnapToTarget" "SnapToTarget" "SnapToTarget" true)
      (Variables|Default|SetAnim (Variables|/Game/blueprints/weapons/Baseweapon_BP.Baseweapon_BP_C|GetAnim (Variables|Default|Getweaponref)))
      (bind _returnvalue_2 (UserInterface|CreateWidget "/Game/UI/Playerhud_WB.Playerhud_WB_C"))
      (bind _output_get_2 (Variables|Default|Setplayerhudref _returnvalue_2))
      (UserInterface|Viewport|AddtoViewport _output_get_2 0)
      (Utilities|FlowControl|DoOnce false
        (:Completed
          (Variables|/Game/blueprints/weapons/Baseweapon_BP.Baseweapon_BP_C|Setcurrentammo (Variables|Default|Getweaponref) (.currentammo _mainweapon))
          (Variables|/Game/blueprints/weapons/Baseweapon_BP.Baseweapon_BP_C|Setmaxammo (Variables|Default|Getweaponref) (.maxammo _mainweapon))
          (while (and (not (Variables|Default|Getissprinting?)) (<= (Variables|Default|Getstamina) 1e+02))
            (Math|Float|IncrementFloat (Variables|Default|Getstamina)))
          (Development|PrintString "STAMINA RECARGADA"))))))

(event EventJumpPortal
  (params (targetLocation :type Vector :default "0, 0, 0") (targetRotation :type Rotator :default "0, 0, 0"))
  ;[0.8697 1 0.04638] Teleport
  (Variables|Default|SetPortal%20Velocity (Math|Vector|VectorLength (Transformation|GetVelocity)))
  (Transformation|SetActorLocationAndRotation targetLocation targetRotation)
  (Pawn|SetControlRotation (Pawn|GetController) targetRotation)
  (Variables|/Script/Engine.MovementComponent|SetVelocity (Variables|Character|GetCharacterMovement) (* (Transformation|GetActorForwardVector) (Variables|Default|GetPortal%20Velocity))))

(event Game|Damage|EventAnyDamage
  (params (Damage :type Float%20%28single-precision%29) (DamageType :type Damage%20Type%20Object%20Reference) (InstigatedBy :type Controller%20Object%20Reference) (DamageCauser :type Actor%20Object%20Reference))
  ;[1 1 1] Damage System
  (if (not (Variables|Default|Getcooldown))
    (bind _output_get (Variables|Default|Sethealth (- (Variables|Default|Gethealth) Damage)))
    (if (<= _output_get 0.0)
      ;;[1 1 1] Show game over when player loses all of there health
      (Utilities|FlowControl|DoOnce false
        (:Completed
          (bind _returnvalue (UserInterface|CreateWidget "/Game/UI/Gameover_WB.Gameover_WB_C"))
          (UserInterface|Viewport|AddtoViewport _returnvalue 0)
          (Pawn|Components|CharacterMovement|DisableMovement (Variables|Character|GetCharacterMovement))))
      (else
        (bind _returnvalue_2 (UserInterface|CreateWidget "/Game/UI/Blood_WB.Blood_WB_C"))
        (UserInterface|Viewport|AddtoViewport _returnvalue_2 0)
        (Default|Updatehealthbar (Variables|Default|Getplayerhudref))
        (Variables|Default|Setcooldown true)
        (Utilities|FlowControl|Delay (Variables|Default|Getcooldowntime))
        (Variables|Default|Setcooldown false)))))

(event Input|KeyboardEvents|DebugKeyF
  (params (Key :type Key%20Structure :default "None") (ActionValue :type Input%20Action%20Value%20Structure))
  (bind _weapon (Variables|Default|Getweapon))
  (bind _returnvalue (Transformation|GetWorldLocation _weapon))
  (:Pressed
    (bind (_outhit _returnvalue_2) (Collision|SphereTraceByChannel (Transformation|GetWorldLocation _weapon) (Math|Vector|MakeVector (+ (.x _returnvalue) 5e+01) (+ (.y _returnvalue) 5e+01) (.z _returnvalue)) 0.0 "TraceTypeQuery1" false 0 "None"))
    (if _returnvalue_2
      (Game|Damage|ApplyDamage 0 15.0 0 0))))

(fn ConstructionScript)

(fn UpdateWeaponSocket
  (bind _weaponref (Variables|Default|Getweaponref))
  (Transformation|AttachComponentToComponent (Variables|/Game/blueprints/weapons/Baseweapon_BP.Baseweapon_BP_C|GetGunmesh _weaponref) (Variables|Default|GetFPSHands) (Variables|/Game/blueprints/weapons/Baseweapon_BP.Baseweapon_BP_C|GetSocket _weaponref) "SnapToTarget" "SnapToTarget" "SnapToTarget" true)
  (Variables|Default|SetAnim (Variables|/Game/blueprints/weapons/Baseweapon_BP.Baseweapon_BP_C|GetAnim _weaponref)))
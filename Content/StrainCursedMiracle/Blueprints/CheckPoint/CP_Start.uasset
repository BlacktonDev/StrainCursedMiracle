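; Start checkpoint that greets the player with a welcome instruction at the beginning of Strain Cursed.
; StartCheckPoint waits briefly, applies depth-of-field blur through the PpVolume post-process settings, and shows the timed message on the first player's HUD.
; After another delay it writes the post-process settings again, apparently to clear the blur.
; BeginPlay, overlap and Tick are unused, so the sequence runs only when StartCheckPoint is called.
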(event EventBeginPlay)

(event Collision|EventActorBeginOverlap
  (params (OtherActor :type Actor%20Object%20Reference)))

(event EventTick
  (params (DeltaSeconds :type Float%20%28single-precision%29)))

(event EventStartCheckPoint
  (bind _pp_volume (Variables|Default|Getpp_Volume))
  (bind _pp_volume_2 (Variables|Default|Getpp_Volume))
  (Utilities|FlowControl|Delay 2.0)
  (Utilities|Struct|SetmembersinPostProcessSettings (Variables|/Script/Engine.PostProcessVolume|GetSettings _pp_volume_2) 2e+02 0.1 1e+01)
  (Variables|/Script/Engine.PostProcessVolume|SetSettings _pp_volume_2 (Variables|/Script/Engine.PostProcessVolume|GetSettings _pp_volume_2))
  (Class|BPIHUD|ShowInstruction(Message) (HUD|GetHUD (Game|GetPlayerController 0)) "Welcom to Strain Cursed" 5.0)
  (Utilities|FlowControl|Delay 4.0)
  (Utilities|Struct|SetmembersinPostProcessSettings (Variables|/Script/Engine.PostProcessVolume|GetSettings _pp_volume) 0.0)
  (Variables|/Script/Engine.PostProcessVolume|SetSettings _pp_volume (Variables|/Script/Engine.PostProcessVolume|GetSettings _pp_volume)))

(fn ConstructionScript
  (|CallParentFunction))
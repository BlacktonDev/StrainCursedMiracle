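; Player character Blueprint for Romo that handles forward and right movement input.
; Each axis event adds movement along the actor's forward or right vector at a fixed scale of 1.0, without using the axis value.
; Rightward movement is skipped while the movement component is flying.
; Both movement paths then call FootstepHeadshake on the player returned by GetPlayer.
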(event EventBeginPlay)

(event Collision|EventActorBeginOverlap
  (params (OtherActor :type Actor%20Object%20Reference)))

(event EventTick
  (params (DeltaSeconds :type Float%20%28single-precision%29)))

(event Input|AxisEvents|InputAxis[HE]MoveForward
  (params (AxisValue :type Float%20%28single-precision%29))
  (Pawn|Input|AddMovementInput (Math|Vector|GetForwardVector (Transformation|GetActorRotation)) 1.0 false)
  (bind _asmaster (CallFunction|GetPlayer))
  (Default|Footstep/Headshake _asmaster "NewEnumerator0"))

(event Input|AxisEvents|InputAxis[HE]MoveRight
  (params (AxisValue :type Float%20%28single-precision%29))
  (if (not (Class|NavMovementComponent|IsFlying (Variables|Character|GetCharacterMovement)))
    (Pawn|Input|AddMovementInput (Math|Vector|GetRightVector (Transformation|GetActorRotation)) 1.0 false)
    (bind _asmaster (CallFunction|GetPlayer))
    (Default|Footstep/Headshake _asmaster "NewEnumerator0")))

(fn ConstructionScript)
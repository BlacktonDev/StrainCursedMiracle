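; PhotoRestore is a short-lived helper actor that rebuilds a saved Cameroid photo from inventory save data.
; Restore strips the leading prefix from the saved photo URL and imports that file as a Texture2D.
; After a brief delay it spawns a CameroidPhotoDeveloped actor, passes it the texture and save data through RetakePhoto, then destroys itself after another short delay.
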(event Custom|Restore
  (params (InventorySave :type Inventory%20Save%20Structure))
  (bind _output_get (Variables|Default|SetDataHolder InventorySave))
  (bind _returnvalue (Class|KismetRenderingLibrary|ImportFileasTexture2D (Utilities|String|GetSubstring (.Photo_Url (Utilities|Struct|BreakInventorySave _output_get)) 8 (Utilities|String|Len (.Photo_Url (Utilities|Struct|BreakInventorySave _output_get))))))
  (Utilities|FlowControl|Delay 0.2)
  (bind _returnvalue_2 (Game|SpawnActorfromClass "/Game/HorrorEngine/Blueprints/UsableAssets/Inventory/CameroidPhotoDeveloped.CameroidPhotoDeveloped_C" (Math|Transform|MakeTransform "0, 0, 0" "0, 0, 0" "1,1,1") "Undefined" 0 0))
  (Default|RetakePhoto _returnvalue_2 _returnvalue (Variables|Default|GetDataHolder))
  (Utilities|FlowControl|Delay 0.2)
  (Actor|DestroyActor))

(fn ConstructionScript)
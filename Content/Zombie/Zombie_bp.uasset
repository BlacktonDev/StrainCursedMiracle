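; Zombie enemy that roams, investigates noises, chases and melees the player, and dies when its health runs out.
; PawnSensing drives AI MoveTo for wandering, noise checks and chasing, with a retriggerable delay returning it to roaming after losing sight.
; An attack hitbox, toggled by CollisionOn/CollisionOff events, damages the player on overlap.
; Death plays a random fall, may drop a health or ammo pickup, and decrements the HUD zombie count.
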(event OnSeePawn(PawnSensing)
  (params (Pawn :type Pawn%20Object%20Reference))
  (if (not (Variables|Default|Getisdead?))
    (Variables|Default|Setseesplayer? true)
    (Utilities|FlowControl|Sequence
      (:then_0
        (AI|AIMoveTo self "0, 0, 0" Pawn 5.0 false
          (:OnSuccess
            (Utilities|FlowControl|DoOnce false :!label _label
              (:Completed
                (bind _returnvalue (Animation|PlayAnimMontage "/Game/Zombie/Mesh/Zombie_Z_Attack_Montage.Zombie_Z_Attack_Montage" 1.0 "None"))
                (Utilities|FlowControl|Delay _returnvalue)
                (goto _label Reset))))))
      (:then_1
        (Utilities|FlowControl|RetriggerableDelay 3.0)
        (Variables|Default|Setseesplayer? false)
        (CallFunction|Roam)))))

(event OnComponentBeginOverlap(zombieattack)
  (params (OverlappedComponent :type Primitive%20Component%20Object%20Reference) (OtherActor :type Actor%20Object%20Reference) (OtherComp :type Primitive%20Component%20Object%20Reference) (OtherBodyIndex :type Integer) (bFromSweep :type Boolean) (SweepResult :type Hit%20Result%20Structure%20%28by%20ref%29))
  (bind _asfpscharacter_bp (Utilities|Casting|CastTofpscharacter_bp OtherActor))
  (Game|Damage|ApplyDamage _asfpscharacter_bp 1e+01 0 0))

(event OnHearNoise(PawnSensing)
  (params (Instigator :type Pawn%20Object%20Reference) (Location :type Vector%20%28by%20ref%29 :default "0, 0, 0") (Volume :type Float%20%28single-precision%29))
  (if (not (or (Variables|Default|Getisdead?) (Variables|Default|Getseesplayer?)))
    (AI|AIMoveTo self Location 0 5.0 false
      (:OnSuccess
        (if (not (or (Variables|Default|Getseesplayer?) (Variables|Default|Getisdead?))) :!label _label
          (AI|AIMoveTo self (.RandomLocation (AI|Navigation|GetRandomReachablePointinRadius (Transformation|GetActorLocation) 5e+02 0 0)) 0 5.0 false
            (:OnSuccess
              (Utilities|FlowControl|Delay 3.0)
              (goto _label))))))))

(event Custom|Roam
  (if (not (or (Variables|Default|Getseesplayer?) (Variables|Default|Getisdead?))) :!label _label
    (AI|AIMoveTo self (.RandomLocation (AI|Navigation|GetRandomReachablePointinRadius (Transformation|GetActorLocation) 5e+02 0 0)) 0 5.0 false
      (:OnSuccess
        (Utilities|FlowControl|Delay 3.0)
        (goto _label)))))

(event Custom|Collision%20On
  (Collision|SetCollisionEnabled (Variables|Default|Getzombieattack) "QueryAndPhysics"))

(event Custom|Collision%20Off
  (Collision|SetCollisionEnabled (Variables|Default|Getzombieattack) "NoCollision"))

(event EventBeginPlay
  (Variables|/Script/Engine.CharacterMovementComponent|SetMaxWalkSpeed (Variables|Character|GetCharacterMovement) (Variables|Default|Getzombiespeed))
  (CallFunction|Roam)
  (Collision|SetCollisionEnabled (Variables|Default|Getzombieattack) "NoCollision"))

(event Collision|EventActorBeginOverlap
  (params (OtherActor :type Actor%20Object%20Reference)))

(event EventTick
  (params (DeltaSeconds :type Float%20%28single-precision%29)))

(event Game|Damage|EventAnyDamage
  (params (Damage :type Float%20%28single-precision%29) (DamageType :type Damage%20Type%20Object%20Reference) (InstigatedBy :type Controller%20Object%20Reference) (DamageCauser :type Actor%20Object%20Reference))
  (bind _returnvalue (Transformation|GetActorTransform))
  (bind _hudref (Variables|Default|GetHudref))
  (if (not (Variables|Default|Getisdead?))
    (bind _output_get (Variables|Default|Sethealth (- (Variables|Default|Gethealth) Damage)))
    (Animation|PlayAnimMontage "/Game/Zombie/Mesh/Zombie_hitreaction_Montage.Zombie_hitreaction_Montage" 1.0 "None")
    (if (<= _output_get 0.0)
      (Utilities|FlowControl|DoOnce false
        (:Completed
          (Variables|Default|Setisdead? true)
          (Components|Movement|StopMovementImmediately (Variables|Character|GetCharacterMovement))
          (Collision|SetCollisionEnabled (Variables|Collision|GetCapsuleComponent) "NoCollision")
          (switch int (Math|Random|RandomIntegerinRange 0 1)
            (:0
              (Animation|PlayAnimMontage "/Game/Zombie/Mesh/Zombie_Z_FallingForward_Montage.Zombie_Z_FallingForward_Montage" 1.0 "None"))
            (:1
              (Animation|PlayAnimMontage "/Game/Zombie/Mesh/Zombie_Z_FallingBack_Montage.Zombie_Z_FallingBack_Montage" 1.0 "None")))
          (switch int (Math|Random|RandomIntegerinRange 0 5)
            (:0
              (Game|SpawnActorfromClass "/Game/blueprints/Objects/Healthpickup_BP.Healthpickup_BP_C" _returnvalue "Undefined" "MultiplyWithRoot" 0 15.0 0))
            (:1
              (Game|SpawnActorfromClass "/Game/blueprints/Objects/Ammopickup_BP.Ammopickup_BP_C" _returnvalue "Undefined" "MultiplyWithRoot" 0 50 0))
            (:2
              _)
            (:3
              _)
            (:4
              _)
            (:5
              _))
          (Utilities|IsValid _hudref
            (:Is%20Valid
              (Math|Integer|DecrementInt (Variables|/Game/UI/Score_WB.Score_WB_C|GetZombies _hudref)
                (:%20%20
                  (Default|Checkzombies _hudref))))
            (:Is%20Not%20Valid
              _))
          (Utilities|FlowControl|Delay 4.0)
          (Actor|DestroyActor))))))

(fn ConstructionScript)